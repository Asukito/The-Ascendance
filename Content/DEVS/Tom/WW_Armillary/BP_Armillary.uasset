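; BP_Armillary is an armillary actor with a gem, a sphere and five rings that are set up to rotate as separate parts.
; Each part has its own RotatingMovement component, bound to it on BeginPlay through SetUpdatedComponent so it can move independently of the others.
; The graph holds no other logic, and the construction script is empty.
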(event EventBeginPlay
  (Components|Movement|SetUpdatedComponent (Variables|Default|GetRotatingMovement_Gem) (Variables|Default|GetArmillary_Gem))
  (Components|Movement|SetUpdatedComponent (Variables|Default|GetRotatingMovement_Sphere) (Variables|Default|GetArmillary_Sphere))
  (Components|Movement|SetUpdatedComponent (Variables|Default|GetRotatingMovement_Ring1) (Variables|Default|GetRing_1))
  (Components|Movement|SetUpdatedComponent (Variables|Default|GetRotatingMovement_Ring2) (Variables|Default|GetRing_2))
  (Components|Movement|SetUpdatedComponent (Variables|Default|GetRotatingMovement_Ring3) (Variables|Default|GetRing_3))
  (Components|Movement|SetUpdatedComponent (Variables|Default|GetRotatingMovement_Ring4) (Variables|Default|GetRing_4))
  (Components|Movement|SetUpdatedComponent (Variables|Default|GetRotatingMovement_Ring5) (Variables|Default|GetRing_5)))

(fn ConstructionScript)